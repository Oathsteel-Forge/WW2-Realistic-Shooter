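; Base character Blueprint providing movement, interaction and inventory, with one equippable component per slot.
; Action events forward to the current equippable through messages, while aiming and sprinting set walk speed and a per-tick head-socket trace finds interactables.
; Slot switches play a montage whose notify re-attaches items between equipped and holstered sockets, and pickups drop any item they replace.
; Left-hand IK uses right-hand bone space to avoid lag, and a capsule trace guards uncrouching.
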(event Custom|Pick%20Up%20Equippable
  (params (EquippableToSpawn :type SMBP%20Equipable%20Item%20Class%20Reference))
  (bind _returnvalue (Transformation|GetActorTransform))
  ;[0.15 0.15 0.15 0.5] Picking Up Items
  (bind _output_get (Variables|Default|SetCurrentEquippedClass (.EquippableClass (Utilities|GetClassDefaults EquippableToSpawn))))
  (bind (_currentequippableoftype _hasequippableoftype) (CallFunction|GetEquipableOfClass _output_get))
  (if _hasequippableoftype
    (Game|SpawnActorfromClass (Variables|/Game/1v1Prototype/Bluprints/SMBP_EquipableItem.SMBP_EquipableItem_C|GetPickUpClass _currentequippableoftype) (Math|Transform|MakeTransform (+ (.location _returnvalue) (* (Math|Vector|GetForwardVector (.rotation _returnvalue)) 2e+01)) "0, 0, 0" "1.000000,1.000000,1.000000") "AdjustIfPossibleButAlwaysSpawn" "MultiplyWithRoot" 0 0)
    (Components|DestroyComponent _currentequippableoftype))
  (bind _returnvalue_2 (Game|AddComponentbyClass EquippableToSpawn false))
  (CallFunction|SetEquippableOfClass (Variables|Default|GetCurrentEquippedClass) _returnvalue_2)
  (Class|BPIEquippable|AddtoInventory(Message) _returnvalue_2 self)
  (Transformation|AttachComponentToComponent _returnvalue_2 (Variables|Character|GetMesh) (Variables|/Game/1v1Prototype/Bluprints/SMBP_EquipableItem.SMBP_EquipableItem_C|GetEquippedSocket _returnvalue_2) "SnapToTarget" "SnapToTarget" "SnapToTarget" true)
  (CallFunction|SetEquippableVisibility))

(event Custom|InteractDelayed
  ;[0.15 0.15 0.15 0.5] Interacting with interactables with a delay (Guns, ammo refill, etc)
  (Class|BPIInteractable|Interact(Message) (Utilities|Array|Get(acopy) (Collision|GetOverlappingActors "/Game/1v1Prototype/Bluprints/Pickups/BP_PickupMaster.BP_PickupMaster_C" :!class /Script/Engine.Actor)) self))

(event Custom|Walk
  ;[0.15 0.15 0.15 0.5] Sprinting/Walking
  (Movement|SetSpeedWalking))

(event Custom|CrouchingEvent
  ;[0.15 0.15 0.15 0.5] Crouching and Uncrouching
  (if (Variables|Default|GetbIsCrouched)
    (if (Animation|CheckSafetoUncouch)
      (Character|UnCrouch))
    (else
      (Character|Crouch))))

(event Custom|StartSecondaryAction
  (bind _currentequippable (CallFunction|GetCurrentEquippable))
  ;[0.15 0.15 0.15 0.5] Secondary Action of Equipped Item (if it has one)
  (if (Utilities|DoesObjectImplementInterface _currentequippable "/Game/1v1Prototype/Bluprints/BPI_ISecondaryActionable.BPI_ISecondaryActionable_C")
    (Class|BPIISecondaryActionable|StartSecondaryAction(Message) _currentequippable)
    (if (Class|GameplayStatics|ObjectIsA _currentequippable "/Game/1v1Prototype/Bluprints/Weapons/FireArms/SMBP_FireArmMaster.SMBP_FireArmMaster_C")
      (Variables|Animation|SetIsAiming true)
      (Movement|SetSpeedAiming))))

(event Custom|StopSecondaryAction
  (bind _currentequippable (CallFunction|GetCurrentEquippable))
  ;[0.15 0.15 0.15 0.5] Secondary Action of Equipped Item (if it has one)
  (if (Utilities|DoesObjectImplementInterface _currentequippable "/Game/1v1Prototype/Bluprints/BPI_ISecondaryActionable.BPI_ISecondaryActionable_C")
    (Class|BPIISecondaryActionable|StopSecondaryAction(Message) _currentequippable)
    (if (Class|GameplayStatics|ObjectIsA _currentequippable "/Game/1v1Prototype/Bluprints/Weapons/FireArms/SMBP_FireArmMaster.SMBP_FireArmMaster_C")
      (Variables|Animation|SetIsAiming false)
      (Movement|SetSpeedWalking))))

(event Custom|StopPrimaryAction
  ;[0.15 0.15 0.15 0.5] Primary Action of Equipped Item
  (Class|BPIEquippable|StopMainAction(Message) (CallFunction|GetCurrentEquippable)))

(event Custom|StartPrimaryAction
  ;[0.15 0.15 0.15 0.5] Primary Action of Equipped Item
  (Class|BPIEquippable|MainAction(Message) (CallFunction|GetCurrentEquippable)))

(event Custom|ReloadEvent
  ;[0.15 0.15 0.15 0.5] Reloading Guns
  (bind _assmbp_fire_arm_master (Utilities|Casting|CastToSMBP_FireArmMaster (CallFunction|GetCurrentEquippable))
    (:then
      (if (Math|Boolean|ANDBoolean (<= (Variables|/Game/1v1Prototype/Bluprints/Weapons/FireArms/SMBP_FireArmMaster.SMBP_FireArmMaster_C|GetCurrentClipAmmo _assmbp_fire_arm_master) (Variables|/Game/1v1Prototype/Bluprints/Weapons/FireArms/SMBP_FireArmMaster.SMBP_FireArmMaster_C|GetClipSize _assmbp_fire_arm_master)) (> (Variables|/Game/1v1Prototype/Bluprints/Weapons/FireArms/SMBP_FireArmMaster.SMBP_FireArmMaster_C|GetReserveAmmo _assmbp_fire_arm_master) 0) (not (Variables|Default|GetIsReloading)))
        (Variables|Default|SetIsReloading true)
        (Default|ReloadEvent _assmbp_fire_arm_master)))
    (:CastFailed
      (Development|PrintString "Not a gun, can't reload"))))

(event Custom|InteractInstant
  (bind _interactableactor (Variables|Default|GetInteractableActor))
  ;[0.15 0.15 0.15 0.5] Interacting with interactables instantly (Doors, windows, etc.)
  (Utilities|IsValid _interactableactor
    (:Is%20Valid
      (Class|BPIInteractable|Interact(Message) _interactableactor self))))

(event Custom|ChangeToPrimary
  ;[0.15 0.15 0.15 0.5] Essentially has character reach behind their back and their currently equiped item will switch out. When deeper into development, need to update to have animations play based on what is being switched out, placing the item where it is to sit when not equipped and have the character reach for the new item they are trying to equip.
  (Variables|Animation|SetShouldLHIK false)
  (if (Utilities|Enum|NotEqual(Enum) (Variables|Default|GetCurrentEquippedClass) "NewEnumerator0")
    (CallFunction|StopSecondaryAction)
    (Variables|Default|SetCanUseEquippable false)
    (Animation|Montage|PlayMontage (Variables|Character|GetMesh) (Variables|Animation|GetSwitchWeaponMontage)
      (:OnCompleted
        (Variables|Animation|SetShouldLHIK true)
        (Variables|Default|SetCanUseEquippable true))
      (:OnNotifyBegin
        (Variables|Default|SetCurrentEquippedClass "NewEnumerator0")
        (CallFunction|SetEquippableVisibility)
        (if (Class|GameplayStatics|ObjectIsA self "/Game/1v1Prototype/Bluprints/Actors/Player/BP_BasePlayer.BP_BasePlayer_C")
          (Default|CallWeaponSwitch))))))

(event Custom|ChangeToSecondary
  ;[0.15 0.15 0.15 0.5] Essentially has character reach behind their back and their currently equiped item will switch out. When deeper into development, need to update to have animations play based on what is being switched out, placing the item where it is to sit when not equipped and have the character reach for the new item they are trying to equip.
  (Variables|Animation|SetShouldLHIK false)
  (if (Utilities|Enum|NotEqual(Enum) (Variables|Default|GetCurrentEquippedClass) "NewEnumerator1")
    (CallFunction|StopSecondaryAction)
    (Variables|Default|SetCanUseEquippable false)
    (Animation|Montage|PlayMontage (Variables|Character|GetMesh) (Variables|Animation|GetSwitchWeaponMontage)
      (:OnCompleted
        (Variables|Animation|SetShouldLHIK true)
        (Variables|Default|SetCanUseEquippable true))
      (:OnNotifyBegin
        (Variables|Default|SetCurrentEquippedClass "NewEnumerator1")
        (CallFunction|SetEquippableVisibility)
        (if (Class|GameplayStatics|ObjectIsA self "/Game/1v1Prototype/Bluprints/Actors/Player/BP_BasePlayer.BP_BasePlayer_C")
          (Default|CallWeaponSwitch))))))

(event Custom|ChangeToMelee
  ;[0.15 0.15 0.15 0.5] Essentially has character reach behind their back and their currently equiped item will switch out. When deeper into development, need to update to have animations play based on what is being switched out, placing the item where it is to sit when not equipped and have the character reach for the new item they are trying to equip.
  (Variables|Animation|SetShouldLHIK false)
  (if (Utilities|Enum|NotEqual(Enum) (Variables|Default|GetCurrentEquippedClass) "NewEnumerator3")
    (CallFunction|StopSecondaryAction)
    (Variables|Default|SetCanUseEquippable false)
    (Animation|Montage|PlayMontage (Variables|Character|GetMesh) (Variables|Animation|GetSwitchWeaponMontage)
      (:OnCompleted
        (Variables|Default|SetCanUseEquippable true))
      (:OnNotifyBegin
        (Variables|Default|SetCurrentEquippedClass "NewEnumerator3")
        (CallFunction|SetEquippableVisibility)
        (if (Class|GameplayStatics|ObjectIsA self "/Game/1v1Prototype/Bluprints/Actors/Player/BP_BasePlayer.BP_BasePlayer_C")
          (Default|CallWeaponSwitch))))))

(event Custom|ChangeToGrenade
  ;[0.15 0.15 0.15 0.5] Essentially has character reach behind their back and their currently equiped item will switch out. When deeper into development, need to update to have animations play based on what is being switched out, placing the item where it is to sit when not equipped and have the character reach for the new item they are trying to equip.
  (Variables|Animation|SetShouldLHIK false)
  (if (Utilities|Enum|NotEqual(Enum) (Variables|Default|GetCurrentEquippedClass) "NewEnumerator5")
    (CallFunction|StopSecondaryAction)
    (Variables|Default|SetCanUseEquippable false)
    (Animation|Montage|PlayMontage (Variables|Character|GetMesh) (Variables|Animation|GetSwitchWeaponMontage)
      (:OnCompleted
        (Variables|Default|SetCanUseEquippable true))
      (:OnNotifyBegin
        (Variables|Default|SetCurrentEquippedClass "NewEnumerator5")
        (CallFunction|SetEquippableVisibility)
        (if (Class|GameplayStatics|ObjectIsA self "/Game/1v1Prototype/Bluprints/Actors/Player/BP_BasePlayer.BP_BasePlayer_C")
          (Default|CallWeaponSwitch))))))

(event Custom|ChangeToSupport
  ;[0.15 0.15 0.15 0.5] Essentially has character reach behind their back and their currently equiped item will switch out. When deeper into development, need to update to have animations play based on what is being switched out, placing the item where it is to sit when not equipped and have the character reach for the new item they are trying to equip.
  (Variables|Animation|SetShouldLHIK false)
  (if (Utilities|Enum|NotEqual(Enum) (Variables|Default|GetCurrentEquippedClass) "NewEnumerator6")
    (CallFunction|StopSecondaryAction)
    (Variables|Default|SetCanUseEquippable false)
    (Animation|Montage|PlayMontage (Variables|Character|GetMesh) (Variables|Animation|GetSwitchWeaponMontage)
      (:OnCompleted
        (Variables|Default|SetCanUseEquippable true))
      (:OnNotifyBegin
        (Variables|Default|SetCurrentEquippedClass "NewEnumerator6")
        (CallFunction|SetEquippableVisibility)
        (if (Class|GameplayStatics|ObjectIsA self "/Game/1v1Prototype/Bluprints/Actors/Player/BP_BasePlayer.BP_BasePlayer_C")
          (Default|CallWeaponSwitch))))))

(event Custom|ChangeToUnarmed
  ;[0.15 0.15 0.15 0.5] Essentially has character reach behind their back and their currently equiped item will switch out. When deeper into development, need to update to have animations play based on what is being switched out, placing the item where it is to sit when not equipped and have the character reach for the new item they are trying to equip.
  (Variables|Animation|SetShouldLHIK false)
  (if (Utilities|Enum|NotEqual(Enum) (Variables|Default|GetCurrentEquippedClass) "NewEnumerator8")
    (CallFunction|StopSecondaryAction)
    (Variables|Default|SetCanUseEquippable false)
    (Animation|Montage|PlayMontage (Variables|Character|GetMesh) (Variables|Animation|GetSwitchWeaponMontage)
      (:OnCompleted
        (Variables|Default|SetCanUseEquippable true))
      (:OnNotifyBegin
        (Variables|Default|SetCurrentEquippedClass "NewEnumerator8")
        (CallFunction|SetEquippableVisibility)
        (if (Class|GameplayStatics|ObjectIsA self "/Game/1v1Prototype/Bluprints/Actors/Player/BP_BasePlayer.BP_BasePlayer_C")
          (Default|CallWeaponSwitch))))))

(event Custom|Sprint
  ;[0.15 0.15 0.15 0.5] Sprinting/Walking
  (Movement|SetSpeedRunning))

(event EventBeginPlay
  (Variables|Movement|SetStandingHalfHeight (Components|Capsule|GetUnscaledCapsuleHalfHeight (Variables|Collision|GetCapsuleComponent))))

(event EventTick
  (params (DeltaSeconds :type Float%20%28single-precision%29))
  (CallFunction|RaycastforInteractable))

(event Input|KeyboardEvents|L
  (params (Key :type Key%20Structure :default "None"))
  (:Pressed
    (Utilities|FlowControl|FlipFlop
      (:A
        (Variables|Animation|SetShouldLHIK true))
      (:B
        (Variables|Animation|SetShouldLHIK false)))))

(fn ConstructionScript)

(fn RaycastforInteractable
  (bind _mesh (Variables|Character|GetMesh))
  (bind _returnvalue (Transformation|GetSocketTransform _mesh "headSocket" "RTS_World"))
  (bind _outhit (Collision|LineTraceByChannel (.location _returnvalue) (+ (.location _returnvalue) (* (Math|Vector|GetForwardVector (.rotation _returnvalue)) "500.000000,500.000000,500.000000")) "TraceTypeQuery1" false 0 "ForOneFrame"))
  (if (Utilities|DoesObjectImplementInterface (.hitactor _outhit) "/Game/1v1Prototype/Bluprints/Interfaces/BPI_Interactable.BPI_Interactable_C")
    (Variables|Default|SetInteractableActor (.hitactor _outhit))
    (else
      (Variables|Default|SetInteractableActor 0))))

(fn GetEquipableOfClass
  (params (EquipbableClass :type Enum_EquipableClass%20Enum :default "NewEnumerator4"))
  (bind _equippables (Variables|Default|GetEquippables))
  (bind (_value _returnvalue) (Utilities|Map|Find _equippables EquipbableClass))
  (return _value _returnvalue))

(fn SetEquippableOfClass
  (params (EquippableClass :type Enum_EquipableClass%20Enum :default "NewEnumerator4") (EquippableToSet :type SMBP%20Equipable%20Item%20Object%20Reference))
  (Utilities|Map|Add (Variables|Default|GetEquippables) EquippableClass EquippableToSet))

(fn GetCurrentEquippable
  (bind _currentequippableoftype (CallFunction|GetEquipableOfClass (Variables|Default|GetCurrentEquippedClass)))
  (return _currentequippableoftype))

(fn SetEquippableVisibility
  (bind _equippables (Variables|Default|GetEquippables))
  (bind _keys (Utilities|Map|Keys _equippables))
  (for _array_element _keys
    (if (Utilities|Enum|NotEqual(Enum) _array_element (Variables|Default|GetCurrentEquippedClass))
      (Utilities|IsValid (.Value (Utilities|Map|Find _equippables _array_element))
        (:Is%20Valid
          (Transformation|AttachComponentToComponent (.Value (Utilities|Map|Find _equippables _array_element)) (Variables|Character|GetMesh) (Variables|/Game/1v1Prototype/Bluprints/SMBP_EquipableItem.SMBP_EquipableItem_C|GetUnEquippedSocket (.Value (Utilities|Map|Find _equippables _array_element))) "KeepRelative" "KeepRelative" "KeepRelative" true)))
      (else
        (Utilities|IsValid (.Value (Utilities|Map|Find _equippables _array_element))
          (:Is%20Valid
            (Transformation|AttachComponentToComponent (.Value (Utilities|Map|Find _equippables _array_element)) (Variables|Character|GetMesh) (Variables|/Game/1v1Prototype/Bluprints/SMBP_EquipableItem.SMBP_EquipableItem_C|GetEquippedSocket (.Value (Utilities|Map|Find _equippables _array_element))) "KeepRelative" "KeepRelative" "KeepRelative" true)))))))

(fn SetSpeedWalking
  (Variables|/Script/Engine.CharacterMovementComponent|SetMaxWalkSpeed (Variables|Character|GetCharacterMovement) (Variables|Movement|GetWalkSpeed)))

(fn SetSpeedRunning
  (Variables|/Script/Engine.CharacterMovementComponent|SetMaxWalkSpeed (Variables|Character|GetCharacterMovement) (Variables|Movement|GetRunSpeed)))

(fn SetSpeedAiming
  (Variables|/Script/Engine.CharacterMovementComponent|SetMaxWalkSpeed (Variables|Character|GetCharacterMovement) (Variables|Movement|GetAimingSpeed)))

(fn GetLHIKTransform
  (bind _currentequippable (CallFunction|GetCurrentEquippable))
  (bind _mesh (Variables|Character|GetMesh))
  (bind _returnvalue (Transformation|GetSocketTransform _currentequippable "LHIK" "RTS_World"))
  (bind (_outposition _outrotation) (Class|SkinnedMeshComponent|TransformtoBoneSpace _mesh "hand_r" (.location _returnvalue) (.rotation _returnvalue)))
  (Utilities|IsValid _currentequippable
    (:Is%20Valid
      (return (Math|Transform|MakeTransform _outposition _outrotation)))))

(fn CheckSafetoUncouch
  (LocalVariables|SetCrouchedHeight (Components|Capsule|GetUnscaledCapsuleHalfHeight (Variables|Collision|GetCapsuleComponent)))
  (LocalVariables|SetStandingHeight (* (Variables|Movement|GetStandingHalfHeight) 2.0))
  (LocalVariables|SetSweepStart (+ (Transformation|GetActorLocation) (Math|Vector|MakeVector 0.0 0.0 (LocalVariables|GetCrouchedHeight))))
  (LocalVariables|SetSweepEnd (+ (Transformation|GetActorLocation) (Math|Vector|MakeVector 0.0 0.0 (LocalVariables|GetStandingHeight))))
  ;[0.15 0.15 0.15 0.5] Check to see if there is something obstructing the player if the uncrouched
  (bind _returnvalue (Collision|CapsuleTraceByChannel (LocalVariables|GetSweepStart) (LocalVariables|GetSweepEnd) (Variables|/Script/Engine.CapsuleComponent|GetCapsuleRadius (Variables|Collision|GetCapsuleComponent)) (Variables|Movement|GetStandingHalfHeight) "TraceTypeQuery1" false 0 "None"))
  (return (not _returnvalue)))

(fn GetFireArmOfType
  (params (FireArmType :type Enum_FireArmType%20Enum :default "NewEnumerator7"))
  (switch Utilities|FlowControl|Switch|SwitchonEnum_FireArmType FireArmType
    (:NewEnumerator7
      (bind (_currentequippableoftype _hasequippableoftype) (CallFunction|GetEquipableOfClass "NewEnumerator0"))
      (if _hasequippableoftype
        (bind _assmbp_fire_arm_master (Utilities|Casting|CastToSMBP_FireArmMaster _currentequippableoftype))
        (return _assmbp_fire_arm_master true)
        (else
          _)))
    (:NewEnumerator9
      (bind (_currentequippableoftype_2 _hasequippableoftype_2) (CallFunction|GetEquipableOfClass "NewEnumerator1"))
      (if _hasequippableoftype_2
        (bind _assmbp_fire_arm_master_2 (Utilities|Casting|CastToSMBP_FireArmMaster _currentequippableoftype_2))
        (return _assmbp_fire_arm_master_2 true)
        (else
          _))))
  (return 0 false))