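; Test AI gunman character that spawns with an MP40, reports combat events to BP_TestAIController and toggles crouching for Cover and Attack.
; BeginPlay sends reload time to the blackboard; low ammo flags a reload.
; Sighted pawns and bullets entering its sphere alert the controller, estimating the shooter's position from reversed bullet velocity at a random distance.
; A capsule hit from a Bullet-tagged actor ragdolls it and stops its brain.
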(event OnSeePawn(PawnSensing)
  (params (Pawn :type Pawn%20Object%20Reference))
  (Default|SeenPawn (Variables|Default|GetAIController) Pawn)
  (Development|PrintString "Saw Something"))

(event OnComponentBeginOverlap(Sphere)
  (params (OverlappedComponent :type Primitive%20Component%20Object%20Reference) (OtherActor :type Actor%20Object%20Reference) (OtherComp :type Primitive%20Component%20Object%20Reference) (OtherBodyIndex :type Integer) (bFromSweep :type Boolean) (SweepResult :type Hit%20Result%20Structure%20%28by%20ref%29))
  ;[0.15 0.15 0.15 0.5] When the NPC gets shot at by anyone (even allied actors)
  (bind _asbp_base_bullet (Utilities|Casting|CastToBP_BaseBullet OtherActor)
    (:then
      (if (!= (Variables|/Game/1v1Prototype/Bluprints/Actors/BP_BaseBullet.BP_BaseBullet_C|GetShooter _asbp_base_bullet) self)
        (bind _prediteddirection (CallFunction|DetermineThreatDirection (Variables|/Script/Engine.MovementComponent|GetVelocity (Variables|/Game/1v1Prototype/Bluprints/Actors/BP_BaseBullet.BP_BaseBullet_C|GetProjectileMovement _asbp_base_bullet))))
        (bind _estimatedposition (CallFunction|EstimateThreatPosition _prediteddirection))
        (Default|Shotat (Variables|Default|GetAIController) _prediteddirection _estimatedposition)))
    (:CastFailed
      (Development|PrintString "Not a bullet"))))

(event OnComponentHit(CapsuleComponent)
  (params (HitComponent :type Primitive%20Component%20Object%20Reference) (OtherActor :type Actor%20Object%20Reference) (OtherComp :type Primitive%20Component%20Object%20Reference) (NormalImpulse :type Vector :default "0, 0, 0") (Hit :type Hit%20Result%20Structure%20%28by%20ref%29))
  (if (Actor|ActorHasTag OtherActor "Bullet")
    (Development|PrintString "Bullet Hit")
    (CallFunction|Ragdoll)))

(event Custom|LowAmmo
  (Default|UpdateBBBool (Variables|Default|GetAIController) "NeedToReload" true))

(event Custom|Ragdoll
  (bind _mesh (Variables|Character|GetMesh))
  (if (Variables|Default|GetIsAlive)
    (Collision|SetCollisionEnabled _mesh "QueryAndPhysics")
    (Physics|SetSimulatePhysics _mesh true)
    (Class|SkeletalMeshComponent|SetPhysicsBlendWeight _mesh 1.0)
    (Variables|Default|SetIsAlive false)
    (Collision|SetCollisionEnabled (Variables|Default|GetCapsuleComponent) "NoCollision")
    (AI|Logic|StopLogic (Variables|/Script/AIModule.AIController|GetBrainComponent (Variables|Default|GetAIController)) "Dead MF")))

(event EventBeginPlay
  (bind _assmbp_fire_arm_master (Utilities|Casting|CastToSMBP_FireArmMaster (Variables|Default|GetEquippedItem)))
  (bind _asbp_test_aicontroller (Utilities|Casting|CastToBP_TestAIController (Pawn|GetController)))
  (Variables|Default|SetAIController _asbp_test_aicontroller)
  (EventDispatchers|BindEventtoAmmoLow _assmbp_fire_arm_master (delegate Custom|LowAmmo))
  (Default|UpdateBBFloat (Variables|Default|GetAIController) "ReloadTime" (Variables|/Game/1v1Prototype/Bluprints/Weapons/FireArms/SMBP_FireArmMaster.SMBP_FireArmMaster_C|GetTimeToReload _assmbp_fire_arm_master)))

(event EventCover
  (bind _asue4asp_hero_tpp_anim_blueprint (Utilities|Casting|CastToUE4ASP_HeroTPP_AnimBlueprint (Components|SkeletalMesh|GetAnimInstance (Variables|Character|GetMesh))))
  (Variables|/Game/AnimStarterPack/UE4ASP_HeroTPP_AnimBlueprint.UE4ASP_HeroTPP_AnimBlueprint_C|SetCrouching _asue4asp_hero_tpp_anim_blueprint true))

(event EventAdvance)

(event EventAttack
  (bind _asue4asp_hero_tpp_anim_blueprint (Utilities|Casting|CastToUE4ASP_HeroTPP_AnimBlueprint (Components|SkeletalMesh|GetAnimInstance (Variables|Character|GetMesh))))
  (Variables|/Game/AnimStarterPack/UE4ASP_HeroTPP_AnimBlueprint.UE4ASP_HeroTPP_AnimBlueprint_C|SetCrouching _asue4asp_hero_tpp_anim_blueprint false))

(fn ConstructionScript
  (CallFunction|TestInitialize))

(fn UpdateWalkSpeed
  (params (NewWalkSpeed :type Float%20%28double-precision%29))
  (Variables|/Script/Engine.CharacterMovementComponent|SetMaxWalkSpeed (Variables|Character|GetCharacterMovement) NewWalkSpeed))

(fn DetermineThreatDirection
  (params (BulletVelocity :type Vector))
  (bind _returnvalue (Math|Vector|Normalize BulletVelocity))
  (bind _returnvalue_2 (Transformation|GetActorLocation))
  (bind _returnvalue_3 (Math|Vector|NegateVector _returnvalue))
  (Rendering|Debug|DrawDebugLine _returnvalue_2 (+ _returnvalue_2 (* _returnvalue_3 "1000.000000,1000.000000,1000.000000")) "(R=0.007146,G=0.000000,B=1.000000,A=1.000000)" 1e+01 1.0)
  (return _returnvalue_3))

(fn EstimateThreatPosition
  (params (ThreatDirection :type Vector))
  (return (+ (* ThreatDirection (Math|Random|RandomFloatinRange 7e+02 1.4e+03)) (.location (Transformation|GetActorTransform self)))))

(fn TestInitialize
  (CallFunction|PickUpEquippable "/Game/1v1Prototype/Bluprints/Weapons/FireArms/PrimaryFireArms/SMGs/SMBP_MP40.SMBP_MP40_C"))