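; Test AI controller that runs BT_TestAI on possess and feeds its blackboard with combat state.
; SeenPawn, meant to be called by the character's pawn sensing, records a Player-tagged target and its location and enters combat.
; ShotAt stores the assumed hostile direction and position; both events start a timer that later clears InCombat.
; AI Perception, look-at rotation and the old lose-player reset are leftover, disconnected logic.
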(event OnTargetPerceptionUpdated(AIPerception)
  (params (Actor :type Actor%20Object%20Reference) (Stimulus :type AI%20Stimulus%20Structure))
  ;[0.15 0.15 0.15 0.5] Outdated. Can't use AI Perception for seeing vertically. Would need to create custom C++ code to do this, which I haven't learned yet and will need time to dive into. For now, using pawn sensing on character BP to take care of this and callsSeen pawn event which takes care of all this logic
)

(event Custom|SeenPawn
  (params (Pawn :type Pawn%20Object%20Reference))
  ;[0.15 0.15 0.15 0.5] Less efficient than AI Perception because constantly has to clear and restart the timer, but serves its purpose for now
  (if (Actor|ActorHasTag Pawn "Player")
    (Utilities|Time|ClearandInvalidateTimerbyHandle (Variables|Default|GetCombatTimer))
    (CallFunction|UpdateValues Pawn)
    (bind _returnvalue (Utilities|Time|SetTimerbyEvent (delegate Custom|ExitCombat) 2e+01))
    (Variables|Default|SetCombatTimer _returnvalue)))

(event Custom|LosePlayer%28old%29
  ;[0.15 0.15 0.15 0.5] Outdated. Can't use AI Perception for seeing vertically. Would need to create custom C++ code to do this, which I haven't learned yet and will need time to dive into. For now, using pawn sensing on character BP to take care of this and callsSeen pawn event which takes care of all this logic
  (CallFunction|ResetCombatBlackboardValues))

(event Custom|ExitCombat
  ;[0.15 0.15 0.15 0.5] Less efficient than AI Perception because constantly has to clear and restart the timer, but serves its purpose for now
  (CallFunction|UpdateBBBool "InCombat" false))

(event Custom|ShotAt
  (params (HostileAssumedDirection :type Vector) (AssumedPosition :type Vector))
  ;[0.15 0.15 0.15 0.5] Shot at by another Actor
  (CallFunction|UpdateBBVector "HostileAssumedDirection" HostileAssumedDirection)
  (CallFunction|UpdateBBVector "HostileAssumedPosition" AssumedPosition)
  (CallFunction|UpdateBBBool "InCombat" true)
  (bind _returnvalue (Utilities|Time|SetTimerbyEvent (delegate Custom|ExitCombat) 2e+01))
  (Variables|Default|SetCombatTimer _returnvalue))

(event EventTick
  (params (DeltaSeconds :type Float%20%28single-precision%29)))

(event EventPossess
  (params (PossessedPawn :type Pawn%20Object%20Reference))
  (AI|RunBehaviorTree "/Game/1v1Prototype/Bluprints/Actors/AI/BT_TestAI.BT_TestAI"))

(fn ConstructionScript)

(fn UpdateValues
  (params (PlayerActor :type Actor%20Object%20Reference))
  (LocalVariables|SetTargetPlayerActor PlayerActor)
  (CallFunction|UpdateBBObject (Utilities|Name|MakeLiteralName "TargetActor") (LocalVariables|GetTargetPlayerActor) false)
  (CallFunction|UpdateBBVector (Utilities|Name|MakeLiteralName "TargetLastKnownLocation") (Transformation|GetActorLocation (LocalVariables|GetTargetPlayerActor)))
  (if (not (ScalableFloat|GetValueasBool (Variables|Default|GetBlackboard) (Utilities|Name|MakeLiteralName "InCombat")))
    (CallFunction|UpdateBBBool (Utilities|Name|MakeLiteralName "InitiatingCombat") true)
    (CallFunction|UpdateBBBool (Utilities|Name|MakeLiteralName "InCombat") true)))

(fn LookatPlayer
  (bind _asactor (Utilities|Casting|CastToActor (AI|Components|Blackboard|GetValueasObject (AI|GetBlackboard 0) (Utilities|Name|MakeLiteralName "TargetActor"))))
  (return (Math|Rotator|FindLookatRotation (.location (Transformation|GetActorTransform (Pawn|GetControlledPawn))) (Transformation|GetActorLocation _asactor))))

(fn UpdateBBObject
  (params (KeyName :type Name) (ObjectValue :type Object%20Object%20Reference) (ShouldClear :type Boolean))
  (bind _blackboard (Variables|Default|GetBlackboard))
  (if ShouldClear
    (AI|Components|Blackboard|ClearValue _blackboard KeyName)
    (else
      (AI|Components|Blackboard|SetValueasObject _blackboard KeyName ObjectValue))))

(fn UpdateBBInt
  (params (KeyName :type Name) (Value :type Integer))
  (Class|BlackboardComponent|SetValueasInt (Variables|Default|GetBlackboard) KeyName Value))

(fn UpdateBBEnum
  (params (KeyName :type Name) (EnumValue :type Byte))
  (AI|Components|Blackboard|SetValueasEnum (Variables|Default|GetBlackboard) KeyName EnumValue))

(fn UpdateBBBool
  (params (KeyName :type Name) (BoolVal :type Boolean))
  (AI|Components|Blackboard|SetValueasBool (Variables|Default|GetBlackboard) KeyName BoolVal))

(fn UpdateBBVector
  (params (KeyName :type Name) (VectorValue :type Vector))
  (AI|Components|Blackboard|SetValueasVector (Variables|Default|GetBlackboard) KeyName VectorValue))

(fn UpdateBBFloat
  (params (Key%20Name :type Name) (Float%20Val :type Float%20%28double-precision%29))
  (AI|Components|Blackboard|SetValueasFloat (Variables|Default|GetBlackboard) Key%20Name Float%20Val))

(fn ResetCombatBlackboardValues
  (CallFunction|UpdateBBInt (Utilities|Name|MakeLiteralName "SearchCount"))
  (CallFunction|UpdateBBObject (Utilities|Name|MakeLiteralName "TargetActor") 0 true)
  (CallFunction|UpdateBBBool (Utilities|Name|MakeLiteralName "InCombat") false)
  (CallFunction|UpdateBBEnum (Utilities|Name|MakeLiteralName "CoverState"))
  (CallFunction|UpdateBBBool (Utilities|Name|MakeLiteralName "ShouldCrouch") false)
  (CallFunction|UpdateBBVector (Utilities|Name|MakeLiteralName "CurrentCoverPosition") "0, 0, 0")
  (CallFunction|UpdateBBVector (Utilities|Name|MakeLiteralName "HostileAssumedDirection") "0, 0, 0")
  (CallFunction|UpdateBBBool (Utilities|Name|MakeLiteralName "InitiatingCombat") false)
  (CallFunction|UpdateBBVector (Utilities|Name|MakeLiteralName "TargetLastKnownLocation") "0, 0, 0"))