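; Ammo box pickup that refills the reserve ammo of the interacting character's primary and secondary guns from a limited shared pool.
; TempInteract runs primary then secondary refill, checking the first two inventory slots for the matching gun class.
; Each refill tops up to max or gives whatever remains, updates the gun's HUD, and destroys the box once empty.
; Remaining ammo is printed on screen as debug output.
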(event EventTempInteract
  (params (InteractingCharacter :type BP%20Base%20Player%20Object%20Reference))
  ;[0.15 0.15 0.15 0.5] Update to only add to he player's primary and secondary ammo
  (CallFunction|RefillPrimaryAmmo InteractingCharacter)
  (CallFunction|RefillSecondaryAmmo InteractingCharacter))

(event EventBeginPlay
  (bind _output_get (Variables|Default|SetCurrentAmmo 60))
  (Development|PrintString (Utilities|String|ToString(Integer) _output_get)))

(fn ConstructionScript)

(fn RefillPrimaryAmmo
  (params (InteractingPlayer :type BP%20Base%20Player%20Object%20Reference))
  (bind _inventory (Variables|/Game/6v6Prototype/Bluprints/Actors/BP_BasePlayer.BP_BasePlayer_C|GetInventory InteractingPlayer))
  (bind _output (Utilities|Array|Get(acopy) _inventory))
  (LocalVariables|SetPlayer 0)
  (Utilities|IsValid _output
    (:Is%20Valid
      (if (Class|GameplayStatics|ObjectIsA _output "/Game/6v6Prototype/Bluprints/Weapons/FireArms/PrimaryFireArms/SMBP_PrimaryGun.SMBP_PrimaryGun_C")
        (bind _assmbp_primary_gun (Utilities|Casting|CastToSMBP_PrimaryGun _output))
        (LocalVariables|SetPrimary _assmbp_primary_gun)
        (bind _output_get (LocalVariables|SetAmmoNeeded (- (Variables|/Game/6v6Prototype/Bluprints/Weapons/FireArms/SMBP_FireArmMaster.SMBP_FireArmMaster_C|GetMaxAmmo _assmbp_primary_gun) (Variables|/Game/6v6Prototype/Bluprints/Weapons/FireArms/SMBP_FireArmMaster.SMBP_FireArmMaster_C|GetReserveAmmo _assmbp_primary_gun))))
        (if (> _output_get 0)
          (if (<= (LocalVariables|GetAmmoNeeded) (Variables|Default|GetCurrentAmmo))
            ;[0.15 0.15 0.15 0.5] If the ammo crate has enough ammo for a full refill
            (Variables|/Game/6v6Prototype/Bluprints/Weapons/FireArms/SMBP_FireArmMaster.SMBP_FireArmMaster_C|SetReserveAmmo (LocalVariables|GetPrimary) (Variables|/Game/6v6Prototype/Bluprints/Weapons/FireArms/SMBP_FireArmMaster.SMBP_FireArmMaster_C|GetMaxAmmo (LocalVariables|GetPrimary)))
            (Variables|Default|SetCurrentAmmo (- (Variables|Default|GetCurrentAmmo) (LocalVariables|GetAmmoNeeded)))
            (else
              ;[0.15 0.15 0.15 0.5] If the ammo crate doesn't have enough ammo for a full refill
              (Variables|/Game/6v6Prototype/Bluprints/Weapons/FireArms/SMBP_FireArmMaster.SMBP_FireArmMaster_C|SetReserveAmmo (LocalVariables|GetPrimary) (+ (Variables|/Game/6v6Prototype/Bluprints/Weapons/FireArms/SMBP_FireArmMaster.SMBP_FireArmMaster_C|GetReserveAmmo (LocalVariables|GetPrimary)) (Variables|Default|GetCurrentAmmo)))
              (Variables|Default|SetCurrentAmmo 0)))
          (Default|UpdateHUD (LocalVariables|GetPrimary))
          (Development|PrintString (Utilities|String|ToString(Integer) (Variables|Default|GetCurrentAmmo)))
          (if (< (Variables|Default|GetCurrentAmmo) 1)
            (Actor|DestroyActor)))))))

(fn RefillSecondaryAmmo
  (params (InteractingPlayer :type BP%20Base%20Player%20Object%20Reference))
  (bind _inventory (Variables|/Game/6v6Prototype/Bluprints/Actors/BP_BasePlayer.BP_BasePlayer_C|GetInventory InteractingPlayer))
  (bind _output (Utilities|Array|Get(acopy) _inventory 1))
  (Utilities|IsValid _output
    (:Is%20Valid
      (if (Class|GameplayStatics|ObjectIsA _output "/Game/6v6Prototype/Bluprints/Weapons/FireArms/SecondaryFireArms/SMBP_SecondaryGun.SMBP_SecondaryGun_C")
        (bind _assmbp_secondary_gun (Utilities|Casting|CastToSMBP_SecondaryGun _output))
        (LocalVariables|SetSecondary _assmbp_secondary_gun)
        (bind _output_get (LocalVariables|SetAmmoNeeded (- (Variables|/Game/6v6Prototype/Bluprints/Weapons/FireArms/SMBP_FireArmMaster.SMBP_FireArmMaster_C|GetMaxAmmo _assmbp_secondary_gun) (Variables|/Game/6v6Prototype/Bluprints/Weapons/FireArms/SMBP_FireArmMaster.SMBP_FireArmMaster_C|GetReserveAmmo _assmbp_secondary_gun))))
        (if (> _output_get 0)
          (if (<= (LocalVariables|GetAmmoNeeded) (Variables|Default|GetCurrentAmmo))
            (Variables|/Game/6v6Prototype/Bluprints/Weapons/FireArms/SMBP_FireArmMaster.SMBP_FireArmMaster_C|SetReserveAmmo (LocalVariables|GetSecondary) (Variables|/Game/6v6Prototype/Bluprints/Weapons/FireArms/SMBP_FireArmMaster.SMBP_FireArmMaster_C|GetMaxAmmo (LocalVariables|GetSecondary)))
            (Variables|Default|SetCurrentAmmo (- (Variables|Default|GetCurrentAmmo) (LocalVariables|GetAmmoNeeded)))
            (else
              (Variables|/Game/6v6Prototype/Bluprints/Weapons/FireArms/SMBP_FireArmMaster.SMBP_FireArmMaster_C|SetReserveAmmo (LocalVariables|GetSecondary) (+ (Variables|/Game/6v6Prototype/Bluprints/Weapons/FireArms/SMBP_FireArmMaster.SMBP_FireArmMaster_C|GetReserveAmmo (LocalVariables|GetSecondary)) (Variables|Default|GetCurrentAmmo)))
              (Variables|Default|SetCurrentAmmo 0)))
          (Default|UpdateHUD (LocalVariables|GetSecondary))
          (Development|PrintString (Utilities|String|ToString(Integer) (Variables|Default|GetCurrentAmmo)))
          (if (< (Variables|Default|GetCurrentAmmo) 1)
            (Actor|DestroyActor)))))))