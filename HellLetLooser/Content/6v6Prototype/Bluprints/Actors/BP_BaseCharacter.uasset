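; Base character for the 6v6 prototype, handling interaction, equippable slots, crouch and movement speeds.
; Each tick a head-socket trace caches the interactable for instant use, while delayed interaction targets an overlapping pickup.
; Equippables are components mapped by slot class; pickups replace the slot's component, spawning the old one's pickup actor.
; Primary actions forward to the current equippable, and slot changes play an equip montage whose notify toggles component visibility.
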(event Custom|Pick%20Up%20Equippable
  (params (EquippableToSpawn :type SMBP%20Equipable%20Item%20Class%20Reference) (Pickup'sLocation :type Vector))
  (bind _returnvalue (Transformation|GetActorTransform))
  ;[0.15 0.15 0.15 0.5] Pickuing Up Items
  (bind _output_get (Variables|Default|SetCurrentEquippedClass (.EquippableClass (Utilities|GetClassDefaults EquippableToSpawn))))
  (bind (_currentequippableoftype _hasequippableoftype) (CallFunction|GetEquipableOfClass _output_get))
  (if _hasequippableoftype
    (Game|SpawnActorfromClass (Variables|/Game/6v6Prototype/Bluprints/SMBP_EquipableItem.SMBP_EquipableItem_C|GetPickUpClass _currentequippableoftype) (Math|Transform|MakeTransform (+ (.location _returnvalue) (* (Math|Vector|GetForwardVector (.rotation _returnvalue)) 2e+01)) "0, 0, 0" "1.000000,1.000000,1.000000") "AdjustIfPossibleButAlwaysSpawn" "MultiplyWithRoot" 0 0)
    (Components|DestroyComponent _currentequippableoftype))
  (bind _returnvalue_2 (Game|AddComponentbyClass EquippableToSpawn false))
  (CallFunction|SetEquippableOfClass (Variables|Default|GetCurrentEquippedClass) _returnvalue_2))

(event Custom|InteractDelayed
  ;[0.15 0.15 0.15 0.5] Interacting with interactables with a delay (Guns, ammo refill, etc)
  (Class|BPIInteractable|Interact(Message) (Utilities|Array|Get(acopy) (Collision|GetOverlappingActors "/Game/6v6Prototype/Bluprints/Pickups/BP_PickupMaster.BP_PickupMaster_C" :!class /Script/Engine.Actor)) self))

(event Custom|Duck
  ;[0.15 0.15 0.15 0.5] Crouching
  (Character|Crouch))

(event Custom|UnDuck
  ;[0.15 0.15 0.15 0.5] Crouching
  (Character|UnCrouch))

(event Custom|StartSecondaryAction
  ;[0.15 0.15 0.15 0.5] Secondary Action of Equipables (if they have one)
  (Variables|Default|SetRightClickActive true))

(event Custom|StopSecondaryAction
  ;[0.15 0.15 0.15 0.5] Secondary Action of Equipables (if they have one)
  (Variables|Default|SetRightClickActive true))

(event Custom|StopPrimaryAction
  ;[0.15 0.15 0.15 0.5] Primary Action
  (bind _currentequippable (CallFunction|GetCurrentEquippable))
  (Class|BPIEquippable|StopMainAction(Message) _currentequippable))

(event Custom|StartPrimaryAction
  ;[0.15 0.15 0.15 0.5] Primary Action
  (bind _currentequippable (CallFunction|GetCurrentEquippable))
  (Default|MainAction _currentequippable))

(event Custom|InteractInstant
  (bind _interactableactor (Variables|Default|GetInteractableActor))
  ;[0.15 0.15 0.15 0.5] Interacting with interactables instantly (Doors, windows, etc.)
  (Utilities|IsValid _interactableactor
    (:Is%20Valid
      (Class|BPIInteractable|Interact(Message) _interactableactor self))))

(event Custom|ChangeToPrimary
  ;[0.15 0.15 0.15 0.5] Essentially has character reach behind their back and their currently equiped item will switch out. When deeper into development, need to update to have animations play based on what is being switched out, placing the item where it is to sit when not equipped and have the character reach for the new item they are trying to equip.
  (if (Utilities|Enum|NotEqual(Enum) (Variables|Default|GetCurrentEquippedClass) "NewEnumerator0")
    (Variables|Default|SetCanUseEquippable false)
    (Variables|Default|SetCurrentEquippedClass "NewEnumerator0")
    (Animation|Montage|PlayMontage (Variables|Character|GetMesh) "/Game/AnimStarterPack/UE5/UE5_Equip_Rifle_Standing_Montage.UE5_Equip_Rifle_Standing_Montage" 1.4
      (:OnCompleted
        (Variables|Default|SetCanUseEquippable true))
      (:OnNotifyBegin
        (CallFunction|SetEquippableVisibility)))))

(event Custom|ChangeToSecondary
  ;[0.15 0.15 0.15 0.5] Essentially has character reach behind their back and their currently equiped item will switch out. When deeper into development, need to update to have animations play based on what is being switched out, placing the item where it is to sit when not equipped and have the character reach for the new item they are trying to equip.
  (Variables|Default|SetCanUseEquippable false)
  (Variables|Default|SetCurrentEquippedClass "NewEnumerator1")
  (Animation|Montage|PlayMontage (Variables|Character|GetMesh) "/Game/AnimStarterPack/UE5/UE5_Equip_Rifle_Standing_Montage.UE5_Equip_Rifle_Standing_Montage" 1.4
    (:OnCompleted
      (Variables|Default|SetCanUseEquippable true))
    (:OnNotifyBegin
      (CallFunction|SetEquippableVisibility))))

(event Custom|ChangeToMelee
  ;[0.15 0.15 0.15 0.5] Essentially has character reach behind their back and their currently equiped item will switch out. When deeper into development, need to update to have animations play based on what is being switched out, placing the item where it is to sit when not equipped and have the character reach for the new item they are trying to equip.
  (if (Utilities|Enum|NotEqual(Enum) (Variables|Default|GetCurrentEquippedClass) "NewEnumerator3")
    (Variables|Default|SetCanUseEquippable false)
    (Variables|Default|SetCurrentEquippedClass "NewEnumerator3")
    (Animation|Montage|PlayMontage (Variables|Character|GetMesh) "/Game/AnimStarterPack/UE5/UE5_Equip_Rifle_Standing_Montage.UE5_Equip_Rifle_Standing_Montage" 1.4
      (:OnCompleted
        (Variables|Default|SetCanUseEquippable true))
      (:OnNotifyBegin
        (CallFunction|SetEquippableVisibility)))))

(event Custom|ChangeToGrenade
  ;[0.15 0.15 0.15 0.5] Essentially has character reach behind their back and their currently equiped item will switch out. When deeper into development, need to update to have animations play based on what is being switched out, placing the item where it is to sit when not equipped and have the character reach for the new item they are trying to equip.
  (if (Utilities|Enum|NotEqual(Enum) (Variables|Default|GetCurrentEquippedClass) "NewEnumerator5")
    (Variables|Default|SetCanUseEquippable false)
    (Variables|Default|SetCurrentEquippedClass "NewEnumerator5")
    (Animation|Montage|PlayMontage (Variables|Character|GetMesh) "/Game/AnimStarterPack/UE5/UE5_Equip_Rifle_Standing_Montage.UE5_Equip_Rifle_Standing_Montage" 1.4
      (:OnCompleted
        (Variables|Default|SetCanUseEquippable true))
      (:OnNotifyBegin
        (CallFunction|SetEquippableVisibility)))))

(event Custom|ChangeToSupport
  ;[0.15 0.15 0.15 0.5] Essentially has character reach behind their back and their currently equiped item will switch out. When deeper into development, need to update to have animations play based on what is being switched out, placing the item where it is to sit when not equipped and have the character reach for the new item they are trying to equip.
  (if (Utilities|Enum|NotEqual(Enum) (Variables|Default|GetCurrentEquippedClass) "NewEnumerator6")
    (Variables|Default|SetCanUseEquippable false)
    (Variables|Default|SetCurrentEquippedClass "NewEnumerator6")
    (Animation|Montage|PlayMontage (Variables|Character|GetMesh) "/Game/AnimStarterPack/UE5/UE5_Equip_Rifle_Standing_Montage.UE5_Equip_Rifle_Standing_Montage" 1.4
      (:OnCompleted
        (Variables|Default|SetCanUseEquippable true))
      (:OnNotifyBegin
        (CallFunction|SetEquippableVisibility)))))

(event Custom|ChangeToUnarmed
  ;[0.15 0.15 0.15 0.5] Essentially has character reach behind their back and their currently equiped item will switch out. When deeper into development, need to update to have animations play based on what is being switched out, placing the item where it is to sit when not equipped and have the character reach for the new item they are trying to equip.
  (if (Utilities|Enum|NotEqual(Enum) (Variables|Default|GetCurrentEquippedClass) "NewEnumerator4")
    (Variables|Default|SetCanUseEquippable false)
    (Variables|Default|SetCurrentEquippedClass "NewEnumerator4")
    (Animation|Montage|PlayMontage (Variables|Character|GetMesh) "/Game/AnimStarterPack/UE5/UE5_Equip_Rifle_Standing_Montage.UE5_Equip_Rifle_Standing_Montage" 1.4
      (:OnCompleted
        (Variables|Default|SetCanUseEquippable true))
      (:OnNotifyBegin
        (CallFunction|SetEquippableVisibility)))))

(event EventBeginPlay)

(event Collision|EventActorBeginOverlap
  (params (OtherActor :type Actor%20Object%20Reference)))

(event EventTick
  (params (DeltaSeconds :type Float%20%28single-precision%29))
  (CallFunction|RaycastforInteractable))

(fn ConstructionScript)

(fn RaycastforInteractable
  (bind _mesh (Variables|Character|GetMesh))
  (bind _returnvalue (Transformation|GetSocketTransform _mesh "headSocket" "RTS_World"))
  (bind _outhit (Collision|LineTraceByChannel (.location _returnvalue) (+ (.location _returnvalue) (* (Math|Vector|GetForwardVector (.rotation _returnvalue)) "500.000000,500.000000,500.000000")) "TraceTypeQuery1" false 0 "None"))
  (if (Utilities|DoesObjectImplementInterface (.hitactor _outhit) "/Game/6v6Prototype/Bluprints/Interfaces/BPI_Interactable.BPI_Interactable_C")
    (Variables|Default|SetInteractableActor (.hitactor _outhit))
    (else
      (Variables|Default|SetInteractableActor 0))))

(fn GetEquipableOfClass
  (params (EquipbableClass :type Enum_EquipableClass%20Enum :default "NewEnumerator4"))
  (bind _equippables (Variables|Default|GetEquippables))
  (bind (_value _returnvalue) (Utilities|Map|Find _equippables EquipbableClass))
  (return _value _returnvalue))

(fn SetEquippableOfClass
  (params (EquippableClass :type Enum_EquipableClass%20Enum :default "NewEnumerator4") (EquippableToSet :type SMBP%20Equipable%20Item%20Object%20Reference))
  (Utilities|Map|Add (Variables|Default|GetEquippables) EquippableClass EquippableToSet))

(fn GetCurrentEquippable
  (bind _currentequippableoftype (CallFunction|GetEquipableOfClass (Variables|Default|GetCurrentEquippedClass)))
  (return _currentequippableoftype))

(fn SetEquippableVisibility
  (bind _equippables (Variables|Default|GetEquippables))
  (bind _keys (Utilities|Map|Keys _equippables))
  (for _array_element _keys
    (if (Utilities|Enum|NotEqual(Enum) _array_element (Variables|Default|GetCurrentEquippedClass))
      (Utilities|IsValid (.Value (Utilities|Map|Find _equippables _array_element))
        (:Is%20Valid
          (Rendering|SetVisibility (.Value (Utilities|Map|Find _equippables _array_element)) false false)))
      (else
        (Utilities|IsValid (.Value (Utilities|Map|Find _equippables _array_element))
          (:Is%20Valid
            (Rendering|SetVisibility (.Value (Utilities|Map|Find _equippables _array_element)) true false)))))))

(fn SetSpeedWalking
  (Variables|/Script/Engine.CharacterMovementComponent|SetMaxWalkSpeed (Variables|Character|GetCharacterMovement) (Variables|Default|GetWalkSpeed)))

(fn SetSpeedRunning
  (Variables|/Script/Engine.CharacterMovementComponent|SetMaxWalkSpeed (Variables|Character|GetCharacterMovement) (Variables|Default|GetRunSpeed)))

(fn SetSpeedAiming
  (Variables|/Script/Engine.CharacterMovementComponent|SetMaxWalkSpeed (Variables|Character|GetCharacterMovement) (Variables|Default|GetAimingSpeed)))