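; Base bullet projectile for combat, with a Cone component for collision and a ProjectileMovement component for flight.
; Collision stays off from construction until InitializeBullet stores damage, team and shooter, launches it along the Cone's up vector at muzzle velocity and enables collision.
; A Cone hit prints the other actor's name, disables collision and destroys the bullet next tick; no damage is applied here.
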(event OnComponentHit(Cone)
  (params (HitComponent :type Primitive%20Component%20Object%20Reference) (OtherActor :type Actor%20Object%20Reference) (OtherComp :type Primitive%20Component%20Object%20Reference) (NormalImpulse :type Vector :default "0, 0, 0") (Hit :type Hit%20Result%20Structure%20%28by%20ref%29))
  (Development|PrintString (Utilities|GetDisplayName OtherActor))
  (Collision|SetCollisionEnabled (Variables|Default|GetCone) "NoCollision")
  (Utilities|FlowControl|DelayUntilNextTick)
  (Actor|DestroyActor))

(event Custom|Initialize%20Bullet
  (params (BaseDamage :type Float%20%28double-precision%29) (TeamID :type Enum_TeamIDs%20Enum :default "NewEnumerator0") (ShotFromObject :type Actor%20Object%20Reference) (MuzzleVeloctiy :type Float%20%28double-precision%29))
  (bind _projectilemovement (Variables|Default|GetProjectileMovement))
  ;[0.15 0.15 0.15 0.5] Bullet initialization with damage, ID, and other needed information
  (Variables|Default|SetBaseDamage BaseDamage)
  (Variables|Default|SetBulletTeam TeamID)
  (Variables|Default|SetShooter ShotFromObject)
  (bind _output_get (Variables|/Script/Engine.ProjectileMovementComponent|SetInitialSpeed _projectilemovement MuzzleVeloctiy))
  (bind _output_get_2 (Variables|/Script/Engine.ProjectileMovementComponent|SetMaxSpeed _projectilemovement _output_get))
  (Variables|/Script/Engine.MovementComponent|SetVelocity _projectilemovement (* _output_get_2 (Math|Vector|GetUpVector (Variables|Default|GetCone))))
  (Collision|SetActorEnableCollision true))

(event Collision|EventHit
  (params (MyComp :type Primitive%20Component%20Object%20Reference) (Other :type Actor%20Object%20Reference) (OtherComp :type Primitive%20Component%20Object%20Reference) (bSelfMoved :type Boolean) (HitLocation :type Vector :default "0, 0, 0") (HitNormal :type Vector :default "0, 0, 0") (NormalImpulse :type Vector :default "0, 0, 0") (Hit :type Hit%20Result%20Structure%20%28by%20ref%29))
  ;[0.15 0.15 0.15 0.5] Destory Bullet
)

(fn ConstructionScript
  (Collision|SetActorEnableCollision false))