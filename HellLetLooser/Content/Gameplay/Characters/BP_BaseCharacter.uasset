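; Base character that handles equippable inventory, item use, interaction, crouching and movement speeds.
; Equippables are components mapped by slot, attached to a hand holder or holstered sockets, with montage notifies timing swaps and hand IK flags set per item.
; Pickup and drop convert between components and pickup actors, carrying firearm ammo across.
; A head-height line trace finds interactables, and a capsule trace checks headroom before uncrouching.
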(event Custom|Pick%20Up%20Equippable
  (params (EquippableToSpawn :type SMBP%20Equipable%20Item%20Class%20Reference) (InteractingPickup :type BP%20Pickup%20Master%20Object%20Reference))
  (bind _equippableclass (Utilities|GetClassDefaults EquippableToSpawn))
  (bind (_currentequippableoftype _hasequippableoftype) (CallFunction|GetEquipableOfClass _equippableclass))
  ;[0.15 0.15 0.15 0.5] Picking Up Items
  ;;[0.15 0.15 0.15 0.5] Check to see if we have a valid equipped item in that slot
  (if _hasequippableoftype
    (Utilities|IsValid _currentequippableoftype
      (:Is%20Valid
        ;;[0.15 0.15 0.15 0.5] Drop the item that was in the slot originally
        (CallFunction|SpawnPickUp (Variables|/Game/Gameplay/WorldObjects/Equippables/SMBP_EquipableItem.SMBP_EquipableItem_C|GetPickUpClass _currentequippableoftype))
        (Default|DestroyComponentEvent _currentequippableoftype))
      (:Is%20Not%20Valid
        _)))
  (CallFunction|AddEquippabletoInventory EquippableToSpawn InteractingPickup))

(event Custom|DropCurrentEquippable
  ;[0.15 0.15 0.15 0.5] Dropping Equippables
  (CallFunction|DropCurrentEquipped))

(event Custom|Walk
  ;[0.15 0.15 0.15 0.5] Sprinting/Walking
  (Movement|SetSpeedWalking))

(event Custom|HitFeedback
  ;[0.15 0.15 0.15 0.5] Play body shot sound if hit a character
  (if (Pawn|IsLocallyControlled)
    (Audio|PlaySound2D "/Game/Assets/Hit_Generic_5-1.Hit_Generic_5-1" 1.0 1.0 0.0 0 0)))

(event Custom|HeadshotFeedback
  ;[0.15 0.15 0.15 0.5] Play headshot sound if headshot a character
  (if (Pawn|IsLocallyControlled)
    (Audio|PlaySound2D "/Game/Assets/Hit_Generic_2-1.Hit_Generic_2-1" 1.0 1.0 0.0 0 0)))

(event Custom|CrouchingEvent
  ;[0.15 0.15 0.15 0.5] Crouching and Uncrouching
  (if (Variables|Default|GetbIsCrouched)
    (if (Animation|CheckSafetoUncouch)
      (Character|UnCrouch))
    (else
      (Character|Crouch))))

(event Custom|StartSecondaryAction
  (bind _currentequippable (CallFunction|GetCurrentEquippable))
  ;[0.15 0.15 0.15 0.5] Secondary Action of Equipped Item (if it has one)
  (if (Variables|Default|GetCanUseEquippable)
    (if (Utilities|DoesObjectImplementInterface _currentequippable "/Game/Gameplay/WorldObjects/Equippables/BPI_ISecondaryActionable.BPI_ISecondaryActionable_C")
      (Class|BPIISecondaryActionable|StartSecondaryAction(Message) _currentequippable)
      (if (Class|GameplayStatics|ObjectIsA _currentequippable "/Game/Gameplay/WorldObjects/Equippables/Weapons/FireArms/SMBP_FireArmMaster.SMBP_FireArmMaster_C")
        (Variables|Animation|SetIsAiming true)
        (Movement|SetSpeedAiming)))))

(event Custom|StopSecondaryAction
  (bind _currentequippable (CallFunction|GetCurrentEquippable))
  ;[0.15 0.15 0.15 0.5] Secondary Action of Equipped Item (if it has one)
  (if (Utilities|DoesObjectImplementInterface _currentequippable "/Game/Gameplay/WorldObjects/Equippables/BPI_ISecondaryActionable.BPI_ISecondaryActionable_C")
    (Class|BPIISecondaryActionable|StopSecondaryAction(Message) _currentequippable)
    (if (Class|GameplayStatics|ObjectIsA _currentequippable "/Game/Gameplay/WorldObjects/Equippables/Weapons/FireArms/SMBP_FireArmMaster.SMBP_FireArmMaster_C")
      (Variables|Animation|SetIsAiming false)
      (Movement|SetSpeedWalking))))

(event Custom|StopPrimaryAction
  ;[0.15 0.15 0.15 0.5] Primary Action of Equipped Item
  (Class|BPIEquippable|StopMainAction(Message) (CallFunction|GetCurrentEquippable)))

(event Custom|StartPrimaryAction
  ;[0.15 0.15 0.15 0.5] Primary Action of Equipped Item
  (if (Variables|Default|GetCanUseEquippable)
    (Class|BPIEquippable|MainAction(Message) (CallFunction|GetCurrentEquippable))))

(event Custom|ReloadEvent
  ;[0.15 0.15 0.15 0.5] Reloading Guns
  (bind _assmbp_fire_arm_master (Utilities|Casting|CastToSMBP_FireArmMaster (CallFunction|GetCurrentEquippable))
    (:then
      (if (Math|Boolean|ANDBoolean (<= (Variables|/Game/Gameplay/WorldObjects/Equippables/Weapons/FireArms/SMBP_FireArmMaster.SMBP_FireArmMaster_C|GetCurrentClipAmmo _assmbp_fire_arm_master) (Variables|/Game/Gameplay/WorldObjects/Equippables/Weapons/FireArms/SMBP_FireArmMaster.SMBP_FireArmMaster_C|GetClipSize _assmbp_fire_arm_master)) (> (Variables|/Game/Gameplay/WorldObjects/Equippables/Weapons/FireArms/SMBP_FireArmMaster.SMBP_FireArmMaster_C|GetReserveAmmo _assmbp_fire_arm_master) 0) (not (Variables|Default|GetIsReloading)))
        (Variables|Default|SetIsReloading true)
        (Default|ReloadEvent _assmbp_fire_arm_master)))
    (:CastFailed
      (Development|PrintString "Not a gun, can't reload"))))

(event Custom|InteractInstant
  (bind _interactableactor (Variables|Default|GetInteractableActor))
  ;[0.15 0.15 0.15 0.5] Interacting with interactables instantly (Doors, windows, etc.)
  (Utilities|IsValid _interactableactor
    (:Is%20Valid
      (Class|BPIInteractable|Interact(Message) _interactableactor self))))

(event Custom|ChangeToPrimary
  ;[0.15 0.15 0.15 0.5] Essentially has character reach behind their back and their currently equiped item will switch out. When deeper into development, need to update to have animations play based on what is being switched out, placing the item where it is to sit when not equipped and have the character reach for the new item they are trying to equip.
  (if (Utilities|Enum|NotEqual(Enum) (Variables|Default|GetCurrentEquippedClass) "NewEnumerator0")
    (Variables|Animation|SetShouldRHIK false)
    (Variables|Animation|SetShouldLHIK false)
    (CallFunction|StopSecondaryAction)
    (Variables|Default|SetCanUseEquippable false)
    (Animation|Montage|PlayMontage (Variables|Character|GetMesh) (Variables|Animation|GetSwitchWeaponMontage)
      (:OnCompleted
        (Default|CallInventorySwitchCompleted)
        (Variables|Animation|SetShouldRHIK true)
        (Variables|Animation|SetShouldLHIK true)
        (Variables|Default|SetCanUseEquippable true))
      (:OnNotifyBegin
        (Variables|Default|SetCurrentEquippedClass "NewEnumerator0")
        (CallFunction|SetEquippableVisibility)
        (if (Class|GameplayStatics|ObjectIsA self "/Game/Gameplay/Characters/Player_FPS/BP_BasePlayer.BP_BasePlayer_C")
          (Default|CallEquippedItemSwitch))))
    (else
      (Default|CallInventorySwitchCompleted))))

(event Custom|ChangeToSecondary
  ;[0.15 0.15 0.15 0.5] Essentially has character reach behind their back and their currently equiped item will switch out. When deeper into development, need to update to have animations play based on what is being switched out, placing the item where it is to sit when not equipped and have the character reach for the new item they are trying to equip.
  (if (Utilities|Enum|NotEqual(Enum) (Variables|Default|GetCurrentEquippedClass) "NewEnumerator1")
    (Variables|Animation|SetShouldRHIK false)
    (Variables|Animation|SetShouldLHIK false)
    (CallFunction|StopSecondaryAction)
    (Variables|Default|SetCanUseEquippable false)
    (Animation|Montage|PlayMontage (Variables|Character|GetMesh) (Variables|Animation|GetSwitchWeaponMontage)
      (:OnCompleted
        (Default|CallInventorySwitchCompleted)
        (Variables|Animation|SetShouldRHIK true)
        (Variables|Animation|SetShouldLHIK true)
        (Variables|Default|SetCanUseEquippable true))
      (:OnNotifyBegin
        (Variables|Default|SetCurrentEquippedClass "NewEnumerator1")
        (CallFunction|SetEquippableVisibility)
        (if (Class|GameplayStatics|ObjectIsA self "/Game/Gameplay/Characters/Player_FPS/BP_BasePlayer.BP_BasePlayer_C")
          (Default|CallEquippedItemSwitch))))
    (else
      (Default|CallInventorySwitchCompleted))))

(event Custom|ChangeToMelee
  ;[0.15 0.15 0.15 0.5] Essentially has character reach behind their back and their currently equiped item will switch out. When deeper into development, need to update to have animations play based on what is being switched out, placing the item where it is to sit when not equipped and have the character reach for the new item they are trying to equip.
  (if (Utilities|Enum|NotEqual(Enum) (Variables|Default|GetCurrentEquippedClass) "NewEnumerator3")
    (Variables|Animation|SetShouldRHIK false)
    (Variables|Animation|SetShouldLHIK false)
    (CallFunction|StopSecondaryAction)
    (Variables|Default|SetCanUseEquippable false)
    (Animation|Montage|PlayMontage (Variables|Character|GetMesh) (Variables|Animation|GetSwitchWeaponMontage)
      (:OnCompleted
        (Default|CallInventorySwitchCompleted)
        (Variables|Default|SetCanUseEquippable true))
      (:OnNotifyBegin
        (Variables|Default|SetCurrentEquippedClass "NewEnumerator3")
        (CallFunction|SetEquippableVisibility)
        (if (Class|GameplayStatics|ObjectIsA self "/Game/Gameplay/Characters/Player_FPS/BP_BasePlayer.BP_BasePlayer_C")
          (Default|CallEquippedItemSwitch))))
    (else
      (Default|CallInventorySwitchCompleted))))

(event Custom|ChangeToGrenade
  ;[0.15 0.15 0.15 0.5] Essentially has character reach behind their back and their currently equiped item will switch out. When deeper into development, need to update to have animations play based on what is being switched out, placing the item where it is to sit when not equipped and have the character reach for the new item they are trying to equip.
  (if (Utilities|Enum|NotEqual(Enum) (Variables|Default|GetCurrentEquippedClass) "NewEnumerator5")
    (Variables|Animation|SetShouldRHIK false)
    (Variables|Animation|SetShouldLHIK false)
    (CallFunction|StopSecondaryAction)
    (Variables|Default|SetCanUseEquippable false)
    (Animation|Montage|PlayMontage (Variables|Character|GetMesh) (Variables|Animation|GetSwitchWeaponMontage)
      (:OnCompleted
        (Default|CallInventorySwitchCompleted)
        (Variables|Default|SetCanUseEquippable true))
      (:OnNotifyBegin
        (Variables|Default|SetCurrentEquippedClass "NewEnumerator5")
        (CallFunction|SetEquippableVisibility)
        (if (Class|GameplayStatics|ObjectIsA self "/Game/Gameplay/Characters/Player_FPS/BP_BasePlayer.BP_BasePlayer_C")
          (Default|CallEquippedItemSwitch))))
    (else
      (Default|CallInventorySwitchCompleted))))

(event Custom|ChangeToSupport
  ;[0.15 0.15 0.15 0.5] Essentially has character reach behind their back and their currently equiped item will switch out. When deeper into development, need to update to have animations play based on what is being switched out, placing the item where it is to sit when not equipped and have the character reach for the new item they are trying to equip.
  (if (Utilities|Enum|NotEqual(Enum) (Variables|Default|GetCurrentEquippedClass) "NewEnumerator6")
    (Variables|Animation|SetShouldRHIK false)
    (Variables|Animation|SetShouldLHIK false)
    (CallFunction|StopSecondaryAction)
    (Variables|Default|SetCanUseEquippable false)
    (Animation|Montage|PlayMontage (Variables|Character|GetMesh) (Variables|Animation|GetSwitchWeaponMontage)
      (:OnCompleted
        (Default|CallInventorySwitchCompleted)
        (Variables|Default|SetCanUseEquippable true))
      (:OnNotifyBegin
        (Variables|Default|SetCurrentEquippedClass "NewEnumerator6")
        (CallFunction|SetEquippableVisibility)
        (if (Class|GameplayStatics|ObjectIsA self "/Game/Gameplay/Characters/Player_FPS/BP_BasePlayer.BP_BasePlayer_C")
          (Default|CallEquippedItemSwitch))))
    (else
      (Default|CallInventorySwitchCompleted))))

(event Custom|ChangeToUnarmed
  ;[0.15 0.15 0.15 0.5] Essentially has character reach behind their back and their currently equiped item will switch out. When deeper into development, need to update to have animations play based on what is being switched out, placing the item where it is to sit when not equipped and have the character reach for the new item they are trying to equip.
  (if (Utilities|Enum|NotEqual(Enum) (Variables|Default|GetCurrentEquippedClass) "NewEnumerator8")
    (Variables|Animation|SetShouldRHIK false)
    (Variables|Animation|SetShouldLHIK false)
    (CallFunction|StopSecondaryAction)
    (Variables|Default|SetCanUseEquippable false)
    (Animation|Montage|PlayMontage (Variables|Character|GetMesh) (Variables|Animation|GetSwitchWeaponMontage)
      (:OnCompleted
        (Default|CallInventorySwitchCompleted)
        (Variables|Default|SetCanUseEquippable true))
      (:OnNotifyBegin
        (Variables|Default|SetCurrentEquippedClass "NewEnumerator8")
        (CallFunction|SetEquippableVisibility)
        (if (Class|GameplayStatics|ObjectIsA self "/Game/Gameplay/Characters/Player_FPS/BP_BasePlayer.BP_BasePlayer_C")
          (Default|CallEquippedItemSwitch))))
    (else
      (Default|CallInventorySwitchCompleted))))

(event Custom|Sprint
  ;[0.15 0.15 0.15 0.5] Sprinting/Walking
  (Movement|SetSpeedRunning))

(event EventBeginPlay
  (bind _outactors (Actor|GetAllActorsOfClass "/Game/Core/BP_GameManager.BP_GameManager_C"))
  (Variables|Default|SetGameManager (Utilities|Array|Get(acopy) _outactors))
  (Variables|Movement|SetStandingHalfHeight (Components|Capsule|GetUnscaledCapsuleHalfHeight (Variables|Collision|GetCapsuleComponent)))
  (CallFunction|ChangetoPrimary))

(event EventTick
  (params (DeltaSeconds :type Float%20%28single-precision%29))
  (CallFunction|RaycastforInteractable))

(fn ConstructionScript
  (Transformation|AttachComponentToComponent (Variables|Default|GetObjectHolder) (Variables|Character|GetMesh) "hand_r" "KeepRelative" "KeepRelative" "KeepRelative" true))

(fn RaycastforInteractable
  (bind _mesh (Variables|Character|GetMesh))
  (bind _returnvalue (Transformation|GetSocketTransform _mesh "head" "RTS_World"))
  (bind _outhit (Collision|LineTraceByChannel (.location _returnvalue) (+ (.location _returnvalue) (* (Transformation|GetActorForwardVector (Pawn|GetController)) "500.000000,500.000000,500.000000")) "TraceTypeQuery1" false 0 "None"))
  (if (Utilities|DoesObjectImplementInterface (.hitactor _outhit) "/Game/Gameplay/WorldObjects/Interactables/BPI_Interactable.BPI_Interactable_C")
    (Variables|Default|SetInteractableActor (.hitactor _outhit))
    (else
      (Variables|Default|SetInteractableActor 0))))

(fn GetEquipableOfClass
  (params (EquipbableClass :type Enum_EquipableClass%20Enum :default "NewEnumerator4"))
  (bind _equippables (Variables|Default|GetEquippables))
  (bind (_value _returnvalue) (Utilities|Map|Find _equippables EquipbableClass))
  (return _value _returnvalue))

(fn SetEquippableOfClass
  (params (EquippableClass :type Enum_EquipableClass%20Enum :default "NewEnumerator4") (EquippableToSet :type SMBP%20Equipable%20Item%20Object%20Reference))
  (Utilities|Map|Add (Variables|Default|GetEquippables) EquippableClass EquippableToSet))

(fn GetCurrentEquippable
  (return (.CurrentEquippableOfType (CallFunction|GetEquipableOfClass (Variables|Default|GetCurrentEquippedClass)))))

(fn SetEquippableVisibility
  (bind _equippables (Variables|Default|GetEquippables))
  (bind _keys (Utilities|Map|Keys _equippables))
  (for _array_element _keys
    (Utilities|IsValid (.Value (Utilities|Map|Find _equippables _array_element)) ; Make sure there is a valid object in the inventory slot
      (:Is%20Valid
        (if (Utilities|Enum|NotEqual(Enum) _array_element (Variables|Default|GetCurrentEquippedClass))
          ;[0.15 0.15 0.15 0.5] If not the item that is equipped, put the item in its unequipped socket on the player mesh
          (Transformation|AttachComponentToComponent (.Value (Utilities|Map|Find _equippables _array_element)) (Variables|Character|GetMesh) (Variables|/Game/Gameplay/WorldObjects/Equippables/SMBP_EquipableItem.SMBP_EquipableItem_C|GetUnEquippedSocket (.Value (Utilities|Map|Find _equippables _array_element))) "KeepRelative" "KeepRelative" "KeepRelative" true)
          (else
            ;[0.15 0.15 0.15 0.5] Attatch the object to the object holder and take the stored transform in the gun an apply it to object holder. This moves and rotates the holder so that the gun appears to be held by the right hand and have the gun oriented properly
            (Transformation|AttachComponentToComponent (.Value (Utilities|Map|Find _equippables _array_element)) (Variables|Default|GetObjectHolder) "None" "KeepRelative" "KeepRelative" "KeepRelative" true)
            (Transformation|SetRelativeTransform (Variables|Default|GetObjectHolder) (Variables|/Game/Gameplay/WorldObjects/Equippables/SMBP_EquipableItem.SMBP_EquipableItem_C|GetObjectHolderAdjustment (CallFunction|GetCurrentEquippable)) false false)))))))

(fn SetSpeedWalking
  (Variables|/Script/Engine.CharacterMovementComponent|SetMaxWalkSpeed (Variables|Character|GetCharacterMovement) (Variables|Movement|GetWalkSpeed)))

(fn SetSpeedRunning
  (Variables|/Script/Engine.CharacterMovementComponent|SetMaxWalkSpeed (Variables|Character|GetCharacterMovement) (Variables|Movement|GetRunSpeed)))

(fn SetSpeedAiming
  (Variables|/Script/Engine.CharacterMovementComponent|SetMaxWalkSpeed (Variables|Character|GetCharacterMovement) (Variables|Movement|GetAimingSpeed)))

(fn GetLHIKTransform
  (bind _currentequippable (CallFunction|GetCurrentEquippable))
  (bind _mesh (Variables|Character|GetMesh))
  (bind _returnvalue (Transformation|GetSocketTransform _currentequippable "LHIK" "RTS_World"))
  (bind (_outposition _outrotation) (Class|SkinnedMeshComponent|TransformtoBoneSpace _mesh "hand_r" (.location _returnvalue) (.rotation _returnvalue)))
  (Utilities|IsValid _currentequippable
    (:Is%20Valid
      (return (Math|Transform|MakeTransform _outposition _outrotation)))))

(fn CheckSafetoUncouch
  (LocalVariables|SetCrouchedHalfHeight (Components|Capsule|GetUnscaledCapsuleHalfHeight (Variables|Collision|GetCapsuleComponent)))
  (LocalVariables|SetStandingHeight (* (Variables|Movement|GetStandingHalfHeight) 2.0))
  (LocalVariables|SetSweepStart (+ (Transformation|GetActorLocation) (Math|Vector|MakeVector 0.0 0.0 (LocalVariables|GetCrouchedHalfHeight))))
  (LocalVariables|SetSweepEnd (+ (- (Transformation|GetActorLocation) (Math|Vector|MakeVector 0.0 0.0 (LocalVariables|GetCrouchedHalfHeight))) (Math|Vector|MakeVector 0.0 0.0 (LocalVariables|GetStandingHeight))))
  ;[0.15 0.15 0.15 0.5] Check to see if there is something obstructing the player if the uncrouched
  (bind _returnvalue (Collision|CapsuleTraceByChannel (LocalVariables|GetSweepStart) (LocalVariables|GetSweepEnd) (Variables|/Script/Engine.CapsuleComponent|GetCapsuleRadius (Variables|Collision|GetCapsuleComponent)) (Variables|Movement|GetStandingHalfHeight) "TraceTypeQuery1" false 0 "None"))
  (return (not _returnvalue)))

(fn GetFireArmOfType
  (params (FireArmType :type Enum_FireArmType%20Enum :default "NewEnumerator7"))
  (bind (_currentequippableoftype _hasequippableoftype) (CallFunction|GetEquipableOfClass "NewEnumerator0"))
  (bind (_currentequippableoftype_2 _hasequippableoftype_2) (CallFunction|GetEquipableOfClass "NewEnumerator1"))
  ;[0.15 0.15 0.15 0.5] As of writing this comment, this is used to fetch and make sure there is a gun equipped in the gun slots. This way the ammo box blueprint can take those firearms and add ammo to their reserves
  (switch Utilities|FlowControl|Switch|SwitchonEnum_FireArmType FireArmType
    (:NewEnumerator7
      (if _hasequippableoftype
        (bind _assmbp_fire_arm_master (Utilities|Casting|CastToSMBP_FireArmMaster _currentequippableoftype) ; Acts as validator
          (:then
            (return _assmbp_fire_arm_master true))
          (:CastFailed
            _))))
    (:NewEnumerator9
      (if _hasequippableoftype_2
        (bind _assmbp_fire_arm_master_2 (Utilities|Casting|CastToSMBP_FireArmMaster _currentequippableoftype_2) ; Acts as validator
          (:then
            (return _assmbp_fire_arm_master_2 true))
          (:CastFailed
            _)))))
  (return 0 false))

(fn SpawnPickUp
  (params (PickUpClass :type BP%20Pickup%20Master%20Class%20Reference))
  (bind _returnvalue (Transformation|GetActorTransform))
  (bind _returnvalue_2 (Game|SpawnActorfromClass PickUpClass (Math|Transform|MakeTransform (+ (.location _returnvalue) (* (Math|Vector|GetForwardVector (.rotation _returnvalue)) 2e+01)) "0, 0, 0" "1.000000,1.000000,1.000000") "Undefined" "MultiplyWithRoot" 0 0))
  ;[0.15 0.15 0.15 0.5] If the pick up that is spawned is a gun, that means we are dropping a gun and must transfer the ammo stats before deleting the static mesh component form of the gun
  (bind _asbp_fire_arm_pickup (Utilities|Casting|CastToBP_FireArmPickup _returnvalue_2))
  (bind _assmbp_fire_arm_master (Utilities|Casting|CastToSMBP_FireArmMaster (CallFunction|GetCurrentEquippable)))
  (Variables|/Game/Gameplay/WorldObjects/Interactables/PickUps/BP_FireArmPickup.BP_FireArmPickup_C|SetCurrentClipAmmo _asbp_fire_arm_pickup (Variables|/Game/Gameplay/WorldObjects/Equippables/Weapons/FireArms/SMBP_FireArmMaster.SMBP_FireArmMaster_C|GetCurrentClipAmmo _assmbp_fire_arm_master))
  (Variables|/Game/Gameplay/WorldObjects/Interactables/PickUps/BP_FireArmPickup.BP_FireArmPickup_C|SetReserveAmmo _asbp_fire_arm_pickup (Variables|/Game/Gameplay/WorldObjects/Equippables/Weapons/FireArms/SMBP_FireArmMaster.SMBP_FireArmMaster_C|GetReserveAmmo _assmbp_fire_arm_master)))

(fn AddEquippabletoInventory
  (params (EquippableToAdd :type SMBP%20Equipable%20Item%20Class%20Reference) (InteractingPickup :type BP%20Pickup%20Master%20Object%20Reference))
  ;[0.15 0.15 0.15 0.5] Create the equippable item component and set the correct inventory slot to that item
  (bind _returnvalue (Game|AddComponentbyClass EquippableToAdd false))
  (CallFunction|SetEquippableOfClass (Variables|/Game/Gameplay/WorldObjects/Equippables/SMBP_EquipableItem.SMBP_EquipableItem_C|GetEquippableClass _returnvalue) _returnvalue)
  (Class|BPIEquippable|AddtoInventory(Message) _returnvalue self) ; Probably should rename. Just assigns owning character to weapon variable
  (CallFunction|SetEquippableVisibility)
  ;[0.15 0.15 0.15 0.5] If item that was picked up is a gun, update the ammo stats.
  (bind _asbp_fire_arm_pickup (Utilities|Casting|CastToBP_FireArmPickup InteractingPickup)
    (:then
      (bind _assmbp_fire_arm_master (Utilities|Casting|CastToSMBP_FireArmMaster _returnvalue)
        (:then
          (Variables|/Game/Gameplay/WorldObjects/Equippables/Weapons/FireArms/SMBP_FireArmMaster.SMBP_FireArmMaster_C|SetCurrentClipAmmo _assmbp_fire_arm_master (Variables|/Game/Gameplay/WorldObjects/Interactables/PickUps/BP_FireArmPickup.BP_FireArmPickup_C|GetCurrentClipAmmo _asbp_fire_arm_pickup))
          (Variables|/Game/Gameplay/WorldObjects/Equippables/Weapons/FireArms/SMBP_FireArmMaster.SMBP_FireArmMaster_C|SetReserveAmmo _assmbp_fire_arm_master (Variables|/Game/Gameplay/WorldObjects/Interactables/PickUps/BP_FireArmPickup.BP_FireArmPickup_C|GetReserveAmmo _asbp_fire_arm_pickup)))
        (:CastFailed
          _)))
    (:CastFailed
      _))
  (Default|CallEquippedItemSwitch))

(fn DropCurrentEquipped
  (bind _currentequippable (CallFunction|GetCurrentEquippable))
  (Utilities|IsValid _currentequippable ; Enusre its a valid object that we can drop.
    (:Is%20Valid
      (LocalVariables|SetItemBeingDropped _currentequippable)
      (CallFunction|SpawnPickUp (Variables|/Game/Gameplay/WorldObjects/Equippables/SMBP_EquipableItem.SMBP_EquipableItem_C|GetPickUpClass _currentequippable)) ; Spawn it's pick up class
      (CallFunction|SetEquippableOfClass (Variables|Default|GetCurrentEquippedClass)) ; Update the inventory slot to have nothing
      ;[0.15 0.15 0.15 0.5] U[date relevant variables for animation purposes as well as HUD purposes
      (Variables|Default|SetCurrentEquippedClass "NewEnumerator8")
      (Variables|Animation|SetShouldRHIK false)
      (Variables|Animation|SetShouldLHIK false)
      (Default|CallEquippedItemSwitch) ; Update HUD
      (Components|DestroyComponent (LocalVariables|GetItemBeingDropped)) ; Destroy the static mesh component. No longer a part of the character or a part of the inventory
    )))

(fn TestInitialize
  (CallFunction|PickUpEquippable "/Game/Gameplay/WorldObjects/Equippables/Weapons/FireArms/PrimaryFireArms/SMGs/SMBP_MP40.SMBP_MP40_C"))