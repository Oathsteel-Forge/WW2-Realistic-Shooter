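; BP_WeaponPickup is an interactable world pickup that gives a weapon to the character that interacts with it.
; On Interact it passes WeaponToSpawn to the character's PickUpEquippable, then destroys itself.
; No check is made that the pickup succeeds, which an author comment flags as still to be added.
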(event EventBeginPlay
  (|CallParentFunction) ; This node is disabled and will not be called.\nDrag off pins to build functionality.
)

(event Collision|EventActorBeginOverlap
  (params (OtherActor :type Actor%20Object%20Reference))
  (|CallParentFunction OtherActor) ; This node is disabled and will not be called.\nDrag off pins to build functionality.
)

(event EventTick
  (params (DeltaSeconds :type Float%20%28single-precision%29))
  (|CallParentFunction DeltaSeconds) ; This node is disabled and will not be called.\nDrag off pins to build functionality.
)

(event EventInteract
  (params (InteractingCharacter :type BP%20Base%20Character%20Object%20Reference))
  ;[0.15 0.15 0.15 0.5] Have character pickup the weapon.
  ; Need to update to check and see if possible
  (Default|PickUpEquippable InteractingCharacter (Variables|Default|GetWeaponToSpawn))
  (Actor|DestroyActor))

(fn ConstructionScript
  (|CallParentFunction))