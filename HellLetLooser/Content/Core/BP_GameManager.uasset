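; Game manager that respawns dead NPCs and players at team spawn points for Allies and Axis.
; BeginPlay sorts every BP_SpawnPoint into a per-team array by TeamID.
; RespawnNPC and RespawnPlayer share identical logic, spawning the dead character's class raised by capsule half-height, restoring its team and spawning a default controller.
; Location and rotation come from separate random picks, which never select the last entry in multi-point arrays.
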(event Custom|RespawnNPC
  (params (DeadCharacter :type BP%20Base%20Character%20Object%20Reference))
  (bind _spawnpoint (CallFunction|GetRandomAllySpawn))
  (bind _spawnpoint_2 (CallFunction|GetRandomAxisSpawn))
  (bind _returnvalue (Utilities|GetClass DeadCharacter))
  (bind _capsulecomponent (Variables|/Script/Engine.Character|GetCapsuleComponent DeadCharacter))
  (bind _returnvalue_2 (Components|Capsule|GetUnscaledCapsuleHalfHeight _capsulecomponent))
  (switch Utilities|FlowControl|Switch|SwitchonEnum_TeamIDs (Variables|/Game/Gameplay/Characters/BP_BaseCharacter.BP_BaseCharacter_C|GetTeamID DeadCharacter)
    (:NewEnumerator0
      (bind _returnvalue_3 (Game|SpawnActorfromClass _returnvalue (Math|Transform|MakeTransform (+ (Transformation|GetActorLocation _spawnpoint) (Math|Vector|MakeVector 0.0 0.0 _returnvalue_2)) (Transformation|GetActorRotation _spawnpoint)) "Undefined" "MultiplyWithRoot" 0 0))
      (Variables|/Game/Gameplay/Characters/BP_BaseCharacter.BP_BaseCharacter_C|SetTeamID _returnvalue_3 "NewEnumerator0")
      (Pawn|SpawnDefaultController _returnvalue_3))
    (:NewEnumerator1
      (bind _returnvalue_4 (Game|SpawnActorfromClass _returnvalue (Math|Transform|MakeTransform (+ (Math|Vector|MakeVector 0.0 0.0 _returnvalue_2) (Transformation|GetActorLocation _spawnpoint_2)) (Transformation|GetActorRotation _spawnpoint_2)) "Undefined" "MultiplyWithRoot" 0 0))
      (Variables|/Game/Gameplay/Characters/BP_BaseCharacter.BP_BaseCharacter_C|SetTeamID _returnvalue_4 "NewEnumerator1")
      (Pawn|SpawnDefaultController _returnvalue_4))))

(event Custom|RespawnPlayer
  (params (DeadCharacter :type BP%20Base%20Character%20Object%20Reference))
  (bind _spawnpoint (CallFunction|GetRandomAllySpawn))
  (bind _spawnpoint_2 (CallFunction|GetRandomAxisSpawn))
  (bind _returnvalue (Utilities|GetClass DeadCharacter))
  (bind _capsulecomponent (Variables|/Script/Engine.Character|GetCapsuleComponent DeadCharacter))
  (bind _returnvalue_2 (Components|Capsule|GetUnscaledCapsuleHalfHeight _capsulecomponent))
  (switch Utilities|FlowControl|Switch|SwitchonEnum_TeamIDs (Variables|/Game/Gameplay/Characters/BP_BaseCharacter.BP_BaseCharacter_C|GetTeamID DeadCharacter)
    (:NewEnumerator0
      (bind _returnvalue_3 (Game|SpawnActorfromClass _returnvalue (Math|Transform|MakeTransform (+ (Transformation|GetActorLocation _spawnpoint) (Math|Vector|MakeVector 0.0 0.0 _returnvalue_2)) (Transformation|GetActorRotation _spawnpoint)) "Undefined" "MultiplyWithRoot" 0 0))
      (Variables|/Game/Gameplay/Characters/BP_BaseCharacter.BP_BaseCharacter_C|SetTeamID _returnvalue_3 "NewEnumerator0")
      (Pawn|SpawnDefaultController _returnvalue_3))
    (:NewEnumerator1
      (bind _returnvalue_4 (Game|SpawnActorfromClass _returnvalue (Math|Transform|MakeTransform (+ (Math|Vector|MakeVector 0.0 0.0 _returnvalue_2) (Transformation|GetActorLocation _spawnpoint_2)) (Transformation|GetActorRotation _spawnpoint_2)) "Undefined" "MultiplyWithRoot" 0 0))
      (Variables|/Game/Gameplay/Characters/BP_BaseCharacter.BP_BaseCharacter_C|SetTeamID _returnvalue_4 "NewEnumerator1")
      (Pawn|SpawnDefaultController _returnvalue_4))))

(event EventBeginPlay
  ;[0.15 0.15 0.15 0.5] Collect all spawn points and sort them into their relative array.
  (bind _outactors (Actor|GetAllActorsOfClass "/Game/Gameplay/BP_SpawnPoint.BP_SpawnPoint_C"))
  (for _array_element _outactors
    (switch Utilities|FlowControl|Switch|SwitchonEnum_TeamIDs (Variables|/Game/Gameplay/BP_SpawnPoint.BP_SpawnPoint_C|GetTeamID _array_element)
      (:NewEnumerator0
        (Utilities|Array|Add (Variables|Default|GetAlliesSpawns) _array_element))
      (:NewEnumerator1
        (Utilities|Array|Add (Variables|Default|GetAxisSpawn) _array_element)))))

(fn ConstructionScript)

(fn GetRandomAxisSpawn
  (return (Utilities|Array|Get(acopy) (Variables|Default|GetAxisSpawn) (Math|Random|RandomInteger (- (Utilities|Array|Length (Variables|Default|GetAxisSpawn)) 1)))))

(fn GetRandomAllySpawn
  (return (Utilities|Array|Get(acopy) (Variables|Default|GetAlliesSpawns) (Math|Random|RandomInteger (- (Utilities|Array|Length (Variables|Default|GetAlliesSpawns)) 1)))))